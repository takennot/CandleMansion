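; Ghost enemy that sends the player back to the level's first found PlayerStart on touching its hit box.
; The overlap plays a kill sound at the ghost, then after a short delay a restart sound at the player controller's location.
; BeginPlay sets narrator and restart audio variables and starts a looping, randomly timed SpinPlayer timer, but that function is empty, its random-yaw logic left disconnected.
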(event `self.ReceiveBeginPlay`
  (set `self.Restart Sounds` "/Game/SFX/SoundCues/RestartSoundCue.RestartSoundCue")
  (set `self.NarratorNameToPlay` "/Game/SFX/SoundCues/GhostSoundCue.GhostSoundCue")
  (set `self.NarratorAudioToPlay` "/Game/SFX/GhostKills.GhostKills")
  (`KismetSystemLibrary.K2_SetTimer` null "SpinPlayer" (`KismetMathLibrary.RandomFloatInRange` 15.0 30.0) true))

(event `self.HitBox.OnComponentBeginOverlap`
  (params (OverlappedComponent :type "PrimitiveComponent Object Reference") (OtherActor :type "Actor Object Reference") (OtherComp :type "PrimitiveComponent Object Reference") (OtherBodyIndex :type Integer) (bFromSweep :type Boolean) (SweepResult :type "HitResult Structure (by ref)"))
  (cast `/Game/FirstPerson/Blueprints/BP_FirstPersonCharacter` OtherActor)
  (bind _outactors (`GameplayStatics.GetAllActorsOfClass` "/Script/Engine.PlayerStart"))
  (`self.K2_SetActorLocation` (`GameplayStatics.GetPlayerCharacter` 0) (`self.K2_GetActorLocation` (`|GetArrayItem` _outactors)) false false)
  (`GameplayStatics.PlaySoundAtLocation` "/Game/SFX/GhostKills.GhostKills" (`self.K2_GetActorLocation` self) (struct) 1.0 1.0 0.0 null null null null)
  (`KismetSystemLibrary.Delay` 1.0)
  (`GameplayStatics.PlaySoundAtLocation` (`self.Restart Sounds`) (`self.K2_GetActorLocation` (`GameplayStatics.GetPlayerController` 0)) (struct) 1.0 1.0 0.0 null null null null))

(fn `SpinPlayer`)

(fn `UserConstructionScript`)