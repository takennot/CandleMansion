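; Patrolling ghost hazard that sends the first-person player back to the first PlayerStart on hitbox overlap, playing a kill sound and a delayed restart sound.
; Tick moves it at constant speed between Point1 and Point2 at its own height when both are valid.
; Otherwise it bounces along world Y from its spawn using frame-rate-dependent steps.
; A looping timer calls SpinPlayer, whose random view-spin logic is disconnected.
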(event `self.HitBox.OnComponentBeginOverlap`
  (params (OverlappedComponent :type "PrimitiveComponent Object Reference") (OtherActor :type "Actor Object Reference") (OtherComp :type "PrimitiveComponent Object Reference") (OtherBodyIndex :type Integer) (bFromSweep :type Boolean) (SweepResult :type "HitResult Structure (by ref)"))
  (cast `/Game/FirstPerson/Blueprints/BP_FirstPersonCharacter` OtherActor)
  (bind _outactors (`GameplayStatics.GetAllActorsOfClass` "/Script/Engine.PlayerStart"))
  (`self.K2_SetActorLocation` (`GameplayStatics.GetPlayerCharacter` 0) (`self.K2_GetActorLocation` (`|GetArrayItem` _outactors)) false false)
  (`GameplayStatics.PlaySoundAtLocation` "/Game/SFX/GhostKills.GhostKills" (`self.K2_GetActorLocation` self) (struct) 1.0 1.0 0.0 null null null null)
  (`KismetSystemLibrary.Delay` 1.0)
  (`GameplayStatics.PlaySoundAtLocation` (`self.Restart Sounds`) (`self.K2_GetActorLocation` (`GameplayStatics.GetPlayerController` 0)) (struct) 1.0 1.0 0.0 null null null null))

(event `self.ReceiveBeginPlay`
  (set `self.Transform` (`self.GetTransform`))
  (set `self.HasMoved` false)
  (set `self.Restart Sounds` "/Game/SFX/SoundCues/RestartSoundCue.RestartSoundCue")
  (set `self.NarratorNameToPlay` "/Game/SFX/SoundCues/GhostSoundCue.GhostSoundCue")
  (set `self.NarratorAudioToPlay` "/Game/SFX/GhostKills.GhostKills")
  (`KismetSystemLibrary.K2_SetTimer` null "SpinPlayer" (`KismetMathLibrary.RandomFloatInRange` 15.0 30.0) true))

(event `self.ReceiveTick`
  (params (DeltaSeconds :type "Float (single-precision)"))
  ;[1 1 1] TICK
  (if (and (`KismetSystemLibrary.IsValid` (`self.Point1`)) (`KismetSystemLibrary.IsValid` (`self.Point2`)))
    (`self.MoveBetweenPoints` DeltaSeconds)
    (else
      (`self.Move`))))

(event `Move`
  (bind _returnvalue (`self.GetTransform`))
  (bind _returnvalue_2 (`self.GetTransform`))
  ;[1 1 1] Move (Ludvig)
  (if (`self.HasMoved`)
    (`self.K2_SetActorTransform` self (`KismetMathLibrary.MakeTransform` (`KismetMathLibrary.MakeVector` (.x (.location _returnvalue_2)) (- (.y (.location _returnvalue_2)) 1.0) (.z (.location _returnvalue_2)))) false false)
    (if (> (.y (.location (`self.Transform`))) (.y (.location (`self.GetTransform`))))
      (set `self.HasMoved` false)
      (`KismetSystemLibrary.LogString` "false!!!"))
    (else
      (`self.K2_SetActorTransform` self (`KismetMathLibrary.MakeTransform` (`KismetMathLibrary.MakeVector` (.x (.location _returnvalue)) (+ (.y (.location _returnvalue)) 1.0) (.z (.location _returnvalue)))) false false)
      (if (> (.y (.location (`self.GetTransform`))) (+ (.y (.location (`self.Transform`))) 500.0))
        (set `self.HasMoved` true)))))

(event `MoveBetweenPoints`
  (params (DeltaTime :type "Float (double-precision)"))
  (bind _returnvalue (`self.GetTransform`))
  (bind _returnvalue_2 (`KismetMathLibrary.MakeVector` (.x (.location _returnvalue)) (.y (.location _returnvalue)) (.z (.location _returnvalue))))
  (bind _returnvalue_3 (`self.GetTransform` (`self.Point2`)))
  (bind _returnvalue_4 (`self.GetTransform` (`self.Point1`)))
  (bind _returnvalue_5 (`KismetMathLibrary.MakeVector` (.x (.location _returnvalue_3)) (.y (.location _returnvalue_3)) (.z (.location _returnvalue))))
  (bind _returnvalue_6 (`KismetMathLibrary.MakeVector` (.x (.location _returnvalue_4)) (.y (.location _returnvalue_4)) (.z (.location _returnvalue))))
  ;[1 1 1] Move between points (Saga)
  (if (`self.GoToPoint1`)
    (`self.K2_SetActorTransform` (`KismetMathLibrary.Conv_VectorToTransform` (`KismetMathLibrary.VInterpTo_Constant` _returnvalue_2 _returnvalue_6 DeltaTime 70.0)))
    (if (`KismetMathLibrary.NearlyEqual_TransformTransform` (`KismetMathLibrary.Conv_VectorToTransform` _returnvalue_2) (`KismetMathLibrary.Conv_VectorToTransform` _returnvalue_6) 0.001 0.001 0.001)
      (set `self.GoToPoint1` false))
    (else
      (`self.K2_SetActorTransform` (`KismetMathLibrary.Conv_VectorToTransform` (`KismetMathLibrary.VInterpTo_Constant` _returnvalue_2 _returnvalue_5 DeltaTime 70.0)))
      (if (`KismetMathLibrary.NearlyEqual_TransformTransform` (`KismetMathLibrary.Conv_VectorToTransform` _returnvalue_2) (`KismetMathLibrary.Conv_VectorToTransform` _returnvalue_5) 0.001 0.001 0.001)
        (set `self.GoToPoint1` true)))))

(fn `SpinPlayer`)

(fn `UserConstructionScript`)