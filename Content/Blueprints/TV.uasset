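; TV Blueprint for what appears to be an interactive prop with narration and switchable audio.
; On BeginPlay it assigns the narrator cue and audio, an interactive sound, and a TV static loop as the original sound.
; An unconnected, never-executed graph holds debug prints and DoOnce-gated logic for swapping the Audio component between interactive and original sounds; Tick and overlap are empty.
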(event `self.ReceiveBeginPlay`
  (set `self.NarratorNameToPlay` "/Game/SFX/SoundCues/TVSoundCue.TVSoundCue")
  (set `self.NarratorAudioToPlay` "/Game/SFX/Thud/Thud_Metalic-ish.Thud_Metalic-ish")
  (set `self.InteractiveSound` "/Game/SFX/Victory/FinishedGame.FinishedGame")
  (set `self.OriginalSound` "/Game/SFX/TV/214757__timbre__like-static-from-old-cheap-portable-analogue-television.214757__timbre__like-static-from-old-cheap-portable-analogue-television"))

(event `self.ReceiveTick`
  (params (DeltaSeconds :type "Float (single-precision)")))

(fn `UserConstructionScript`)