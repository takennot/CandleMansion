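; Candle actor Blueprint that starts lit and can be put out through an Extinguish function.
; BeginPlay sets the lit flag and assigns a Thud narrator clip along with its name, CandleSoundCue.
; Extinguish, if the candle is lit, deactivates the Niagara effect, plays a blow-out sound, stops the near and far audio loops and returns true.
; If already out, it returns false.
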(event `self.ReceiveBeginPlay`
  (set `self.IsLit` true)
  (set `self.NarratorAudioToPlay` "/Game/SFX/Thud/thud.thud")
  (set `self.NarratorNameToPlay` "/Game/SFX/SoundCues/CandleSoundCue.CandleSoundCue"))

(fn `Extinguish`
  (returns (Extinguished :type Boolean))
  (bind _islit (`self.IsLit`))
  (`|ExecutionSequence`
    (:`then_0`
      (if _islit
        (`ActorComponent.Deactivate` (`self.Niagara`))
        (`GameplayStatics.PlaySoundAtLocation` "/Game/SFX/Furniture/CandleOut/CandleOut.CandleOut" (0.0 0.0 0.0) (struct) 1.0 1.0 0.0 null null null null)
        (`AudioComponent.Stop` (`self.AudioFar`))
        (`AudioComponent.Stop` (`self.AudioClose`))
        (set `self.IsLit` false)
        (return true)
        (else
          (return _islit))))))

(fn `UserConstructionScript`)