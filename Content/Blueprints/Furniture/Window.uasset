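; Window furniture Blueprint that supplies narrator audio and plays a rustling cloth sound.
; On BeginPlay it fills the narrator name and audio variables with the window sound cue and glass knock.
; RUSTLE plays the cloth sound through the Audio component.
; A separate F key handler plays it at the actor's location with attenuation, and both paths print a debug string.
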(event `self.ReceiveBeginPlay`
  (set `self.NarratorNameToPlay` "/Game/SFX/SoundCues/WindowSoundCue.WindowSoundCue")
  (set `self.NarratorAudioToPlay` "/Game/SFX/Thud/glass-knock.glass-knock"))

(event `Key|F` :overrideparent false
  (params (Key :type "Key Structure"))
  (:`Pressed`
    (`KismetSystemLibrary.PrintString` "WINDOWBLOWWW")
    (`GameplayStatics.PlaySoundAtLocation` "/Game/SFX/Attenuations/RustlingCloth.RustlingCloth" (`self.K2_GetActorLocation`) (struct) 1.0 1.0 0.0 "/Game/SFX/Attenuations/RustlingAttenuation.RustlingAttenuation" null null null)))

(fn `RUSTLE`
  (locals (NewLocalVar :type "AudioComponent Object Reference"))
  (bind _audio (`self.Audio`))
  (`KismetSystemLibrary.PrintString` "WINDOWBLOWWW")
  (`AudioComponent.SetSound` _audio "/Game/SFX/Attenuations/RustlingCloth.RustlingCloth")
  (`AudioComponent.Play` _audio 0.0))

(fn `UserConstructionScript`)