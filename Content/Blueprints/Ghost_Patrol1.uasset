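; Patrolling ghost hazard that sends the player back to the first PlayerStart when they touch its hit box, playing a kill sound, then a restart sound.
; Tick shuttles it along world Y between its spawn point and 500 units beyond, one unit per frame, so speed depends on frame rate.
; A randomized looping timer calls an empty SpinPlayer, whose rotation logic is disconnected; the point-to-point movement event is unfinished and uncalled here.
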(event `self.HitBox.OnComponentBeginOverlap`
  (params (OverlappedComponent :type "PrimitiveComponent Object Reference") (OtherActor :type "Actor Object Reference") (OtherComp :type "PrimitiveComponent Object Reference") (OtherBodyIndex :type Integer) (bFromSweep :type Boolean) (SweepResult :type "HitResult Structure (by ref)"))
  (cast `/Game/FirstPerson/Blueprints/BP_FirstPersonCharacter` OtherActor)
  (bind _outactors (`GameplayStatics.GetAllActorsOfClass` "/Script/Engine.PlayerStart"))
  (`self.K2_SetActorLocation` (`GameplayStatics.GetPlayerCharacter` 0) (`self.K2_GetActorLocation` (`|GetArrayItem` _outactors)) false false)
  (`GameplayStatics.PlaySoundAtLocation` "/Game/SFX/GhostKills.GhostKills" (`self.K2_GetActorLocation` self) (struct) 1.0 1.0 0.0 null null null null)
  (`KismetSystemLibrary.Delay` 1.0)
  (`GameplayStatics.PlaySoundAtLocation` (`self.Restart Sounds`) (`self.K2_GetActorLocation` (`GameplayStatics.GetPlayerController` 0)) (struct) 1.0 1.0 0.0 null null null null))

(event `self.ReceiveBeginPlay`
  (set `self.Transform` (`self.GetTransform`))
  (set `self.HasMoved` false)
  (set `self.Restart Sounds` "/Game/SFX/SoundCues/RestartSoundCue.RestartSoundCue")
  (set `self.NarratorNameToPlay` "/Game/SFX/SoundCues/GhostSoundCue.GhostSoundCue")
  (set `self.NarratorAudioToPlay` "/Game/SFX/GhostKills.GhostKills")
  (`KismetSystemLibrary.K2_SetTimer` null "SpinPlayer" (`KismetMathLibrary.RandomFloatInRange` 15.0 30.0) true))

(event `self.ReceiveTick`
  (params (DeltaSeconds :type "Float (single-precision)"))
  (`self.Move`))

(event `Move`
  (bind _returnvalue (`self.GetTransform`))
  (bind _returnvalue_2 (`self.GetTransform`))
  ;[1 1 1] Move (Ludvig)
  (if (`self.HasMoved`)
    (`self.K2_SetActorTransform` self (`KismetMathLibrary.MakeTransform` (`KismetMathLibrary.MakeVector` (.x (.location _returnvalue)) (- (.y (.location _returnvalue)) 1.0) (.z (.location _returnvalue)))) false false)
    (if (> (.y (.location (`self.Transform`))) (.y (.location (`self.GetTransform`))))
      (set `self.HasMoved` false)
      (`KismetSystemLibrary.LogString` "false!!!"))
    (else
      (`self.K2_SetActorTransform` self (`KismetMathLibrary.MakeTransform` (`KismetMathLibrary.MakeVector` (.x (.location _returnvalue_2)) (+ (.y (.location _returnvalue_2)) 1.0) (.z (.location _returnvalue_2)))) false false)
      (if (> (.y (.location (`self.GetTransform`))) (+ (.y (.location (`self.Transform`))) 500.0))
        (set `self.HasMoved` true)))))

(event `MoveBetweenPoints`
  (bind _returnvalue (`self.GetTransform`))
  (bind _returnvalue_2 (`SceneComponent.GetRelativeTransform` (`self.Point1`)))
  (if (`self.GoToPoint1`)
    (`self.K2_SetActorTransform` (`KismetMathLibrary.TLerp` _returnvalue_2 _returnvalue))
    (if (`KismetMathLibrary.NearlyEqual_TransformTransform` _returnvalue _returnvalue_2 0.001 0.001 0.001)
      _)
    (else
      (`self.K2_SetActorTransform` (`KismetMathLibrary.TLerp` (`SceneComponent.GetRelativeTransform` (`self.Point2`)) _returnvalue)))))

(fn `SpinPlayer`)

(fn `UserConstructionScript`)